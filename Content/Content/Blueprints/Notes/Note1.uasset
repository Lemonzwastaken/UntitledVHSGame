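; Note1 is an interactable note pickup that the player can read.
; On Interact it plays a pickup sound at the note mesh, shows the WBP_Note1 widget and switches the player to UI-only input with the cursor hidden.
; CanInteract and InteractPrompt functions expose whether it can be used and supply its prompt flag and name to the interaction system.
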(event `/Game/Content/Blueprints/Interface/BP_Interact.Interact`
  (params (Player :type "/Game/Content/Blueprints/Player/Blueprints/BP_Player Object Reference"))
  (bind _returnvalue (`GameplayStatics.GetPlayerController` 0))
  ; PickupNote
  (`GameplayStatics.PlaySoundAtLocation` "/Game/Content/Assets/Audio/Abilitys/Note/SW_NotePickup.SW_NotePickup" (`SceneComponent.K2_GetComponentLocation` (`self.Note`)) (struct) 1.0 1.0 0.0 null null null null)
  (bind _returnvalue_2 (`|CreateWidget` "/Game/Content/Blueprints/Widgets/NoteSystem/Note1/WBP_Note1.WBP_Note1_C"))
  (`UserWidget.AddToViewport` _returnvalue_2 0)
  (`WidgetBlueprintLibrary.SetInputMode_UIOnlyEx` _returnvalue null)
  (set `PlayerController.bShowMouseCursor` false _returnvalue))

(fn `Can_Interact?`
  (returns (`CanInteract?` :type Boolean))
  (return (`self.CanInteract?`)))

(fn `Interact_Prompt`
  (returns (`ShowPrompt?` :type Boolean) (Name :type Name))
  (return (`self.ShowNotePrompt`) (`self.NoteName`)))

(fn `UserConstructionScript`)